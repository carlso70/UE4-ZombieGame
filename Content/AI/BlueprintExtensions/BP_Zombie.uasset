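; BP_Zombie is a Blueprint extension that handles zombie combat feedback through attack, death and blood-hit events.
; Attack plays a hit-react animation on the passed-in zombie and immediately damages the target player by the zombie's attack damage.
; Die stops the current montage, plays a death animation, resets its own time dilation, spawns a blood decal, then destroys the zombie after a delay.
; SpawnBlood emits a blood particle effect at the hit location.
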(event EventSpawnBlood
  (params (Zombie :type Zombie%20Object%20Reference) (HitLocation :type Vector))
  ;[1 1 1] Blood On Bullet hit
  (Effects|SpawnEmitteratLocation "/Game/Materials/Blood/FXVillesBloodVFXPack/Particles/PS_Blood_BulletHit.PS_Blood_BulletHit" HitLocation))

(event EventAttack
  (params (PlayerToAttack :type Zombie%20Invasion%20Character%20Object%20Reference) (Zombie :type Zombie%20Object%20Reference))
  ;[1 1 1] Zombie attack animation then damage
  (Components|Animation|PlayAnimation (Variables|/Script/Engine.Character|GetMesh Zombie) "/Game/AnimStarterPack/Hit_React_1.Hit_React_1" false)
  (Class|ZombieInvasionCharacter|Damage PlayerToAttack (Variables|/Script/ZombieInvasion.Zombie|GetAttackDamage Zombie)))

(event EventBeginPlay)

(event EventActorBeginOverlap
  (params (OtherActor :type Actor%20Object%20Reference)))

(event EventTick
  (params (DeltaSeconds :type Float%20%28single-precision%29)))

(event EventDie
  (params (Zombie :type Zombie%20Object%20Reference))
  ;[1 1 1] On Death BP_Die()
  (bind _returnvalue (Animation|GetCurrentMontage Zombie :!class /Script/Engine.Character))
  (Animation|StopAnimMontage Zombie _returnvalue)
  (Components|Animation|PlayAnimation (Variables|/Script/Engine.Character|GetMesh Zombie) "/Game/AnimStarterPack/Death_1.Death_1" false)
  (Variables|Default|SetCustomTimeDilation 1.0)
  (Rendering|Decal|SpawnDecalatLocation "/Game/Materials/Blood/BloodSplat1.BloodSplat1" "100.000000,100.000000,100.000000" (Transformation|GetActorLocation Zombie) "-90.000000,0.000000,0.000000" 0.0)
  (Utilities|FlowControl|Delay 5.0)
  (Actor|DestroyActor Zombie))

(fn ConstructionScript)